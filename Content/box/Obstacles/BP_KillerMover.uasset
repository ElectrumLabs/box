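; BP_KillerMover is a moving obstacle that kills the player character on contact.
; On BeginPlay it uses AI MoveTo toward MoveToBeacon.
; A hit or Sphere overlap with BP_MainCharacter destroys the character, shows WBP_DeathScreen and switches to UI input through the game instance.
; An older timer-driven back-and-forth X movement of the Cylinder remains, but its setup is disconnected and never runs.
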(event OnComponentBeginOverlap(Sphere)
  (params (OverlappedComponent :type Primitive%20Component%20Object%20Reference) (OtherActor :type Actor%20Object%20Reference) (OtherComp :type Primitive%20Component%20Object%20Reference) (OtherBodyIndex :type Integer) (bFromSweep :type Boolean) (SweepResult :type Hit%20Result%20Structure%20%28by%20ref%29))
  (bind _asbp_main_character (Utilities|Casting|CastToBP_MainCharacter OtherActor))
  (Actor|DestroyActor _asbp_main_character)
  (bind _returnvalue (UserInterface|CreateWidget "/Game/box/UserInterface/WBP_DeathScreen.WBP_DeathScreen_C" (Game|GetPlayerController 0)))
  (UserInterface|Viewport|AddtoViewport _returnvalue 0)
  (Default|ChangetoUIInput (.AsGI%20Box%20GI (Utilities|Casting|CastToGI_boxGI (Game|GetGameInstance)))))

(event Custom|TransformX
  (bind _cylinder (Variables|Default|GetCylinder))
  (bind _movexrate (Variables|Default|GetMoveXRate))
  (bind _returnvalue (Transformation|GetWorldLocation _cylinder))
  (bind _returnvalue_2 (+ (.x _returnvalue) _movexrate))
  ;[1 1 1] Going forward
  (if (>= _returnvalue_2 (Variables|Default|GetMoveX))
    (Variables|Default|SetbGoForward false)
    (else
      (Transformation|SetWorldLocation (Variables|Default|GetCylinder) (Math|Vector|MakeVector _returnvalue_2 (.y _returnvalue) (.z _returnvalue)) false false))))

(event Custom|ReverseX
  (bind _cylinder (Variables|Default|GetCylinder))
  (bind _movexrate (Variables|Default|GetMoveXRate))
  (bind _returnvalue (Transformation|GetWorldLocation _cylinder))
  (bind _returnvalue_2 (- (.x _returnvalue) _movexrate))
  ;[1 1 1] Going backwards
  (if (<= _returnvalue_2 (Variables|Default|GetOriginX))
    (Variables|Default|SetbGoForward true)
    (else
      (Transformation|SetWorldLocation (Variables|Default|GetCylinder) (Math|Vector|MakeVector _returnvalue_2 (.y _returnvalue) (.z _returnvalue)) false false))))

(event Custom|DirectionHandling
  (if (Variables|Default|GetbGoForward)
    (CallFunction|TransformX)
    (else
      (CallFunction|ReverseX))))

(event EventBeginPlay
  (AI|AIMoveTo 0 "0, 0, 0" (Variables|Default|GetMoveToBeacon) 5.0 false))

(event Collision|EventHit
  (params (MyComp :type Primitive%20Component%20Object%20Reference) (Other :type Actor%20Object%20Reference) (OtherComp :type Primitive%20Component%20Object%20Reference) (bSelfMoved :type Boolean) (HitLocation :type Vector :default "0, 0, 0") (HitNormal :type Vector :default "0, 0, 0") (NormalImpulse :type Vector :default "0, 0, 0") (Hit :type Hit%20Result%20Structure%20%28by%20ref%29))
  (bind _asbp_main_character (Utilities|Casting|CastToBP_MainCharacter Other))
  (Actor|DestroyActor _asbp_main_character)
  (bind _returnvalue (UserInterface|CreateWidget "/Game/box/UserInterface/WBP_DeathScreen.WBP_DeathScreen_C" (Game|GetPlayerController 0)))
  (UserInterface|Viewport|AddtoViewport _returnvalue 0)
  (Default|ChangetoUIInput (.AsGI%20Box%20GI (Utilities|Casting|CastToGI_boxGI (Game|GetGameInstance)))))

(fn ConstructionScript)