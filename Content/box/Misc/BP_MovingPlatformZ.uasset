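; Moving platform actor that oscillates vertically along world Z between its starting height and a configurable MoveZ offset.
; BeginPlay converts the offset to an absolute height and starts a looping timer at RefreshRate, used instead of Tick.
; Each timer call steps the Platform by MoveZRate, flipping GoForward when the next step would reach a limit.
; TransformX and ReverseX handle up and down movement on Z, despite their names.
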(event Custom|TransformX
  (bind _platform (Variables|Default|GetPlatform))
  (bind _movezrate (Variables|Default|GetMoveZRate))
  (bind _returnvalue (Transformation|GetWorldLocation _platform))
  (bind _returnvalue_2 (+ (.z _returnvalue) _movezrate))
  ;[1 1 1] Going forward
  (if (>= _returnvalue_2 (Variables|Default|GetMoveZ))
    (Variables|Default|SetbGoForward false)
    (else
      (Transformation|SetWorldLocation (Variables|Default|GetPlatform) (Math|Vector|MakeVector (.x _returnvalue) (.y _returnvalue) _returnvalue_2) false false))))

(event Custom|ReverseX
  (bind _movezrate (Variables|Default|GetMoveZRate))
  (bind _platform (Variables|Default|GetPlatform))
  (bind _returnvalue (Transformation|GetWorldLocation _platform))
  (bind _returnvalue_2 (- (.z _returnvalue) _movezrate))
  ;[1 1 1] Going backwards
  (if (<= _returnvalue_2 (Variables|Default|GetOriginZ))
    (Variables|Default|SetbGoForward true)
    (else
      (Transformation|SetWorldLocation (Variables|Default|GetPlatform) (Math|Vector|MakeVector (.x _returnvalue) (.y _returnvalue) _returnvalue_2) false false))))

(event Custom|DirectionHandling
  (if (Variables|Default|GetbGoForward)
    (CallFunction|TransformX)
    (else
      (CallFunction|ReverseX))))

(event EventBeginPlay
  (bind _platform (Variables|Default|GetPlatform))
  (bind _returnvalue (Transformation|GetWorldLocation _platform))
  (Variables|Default|SetOriginZ (.z _returnvalue))
  (Variables|Default|SetMoveZ (+ (Variables|Default|GetMoveZ) (.z _returnvalue)))
  (Utilities|Time|SetTimerbyEvent (delegate Custom|DirectionHandling) (Variables|Default|GetRefreshRate) true))

(fn ConstructionScript)