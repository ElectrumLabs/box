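; A moving platform Blueprint that shuttles its Platform component back and forth along the world X axis.
; BeginPlay records the starting X, converts MoveX into a world-space end point, and starts a looping timer at RefreshRate instead of using Tick.
; Each timer call steps the platform by MoveXRate, flipping GoForward when the next step would reach or pass either limit.
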(event Custom|TransformX
  (bind _platform (Variables|Default|GetPlatform))
  (bind _movexrate (Variables|Default|GetMoveXRate))
  (bind _returnvalue (Transformation|GetWorldLocation _platform))
  (bind _returnvalue_2 (+ (.x _returnvalue) _movexrate))
  ;[1 1 1] Going forward
  (if (>= _returnvalue_2 (Variables|Default|GetMoveX))
    (Variables|Default|SetbGoForward false)
    (else
      (Transformation|SetWorldLocation (Variables|Default|GetPlatform) (Math|Vector|MakeVector _returnvalue_2 (.y _returnvalue) (.z _returnvalue)) false false))))

(event Custom|ReverseX
  (bind _movexrate (Variables|Default|GetMoveXRate))
  (bind _platform (Variables|Default|GetPlatform))
  (bind _returnvalue (Transformation|GetWorldLocation _platform))
  (bind _returnvalue_2 (- (.x _returnvalue) _movexrate))
  ;[1 1 1] Going backwards
  (if (<= _returnvalue_2 (Variables|Default|GetOriginX))
    (Variables|Default|SetbGoForward true)
    (else
      (Transformation|SetWorldLocation (Variables|Default|GetPlatform) (Math|Vector|MakeVector _returnvalue_2 (.y _returnvalue) (.z _returnvalue)) false false))))

(event Custom|DirectionHandling
  (if (Variables|Default|GetbGoForward)
    (CallFunction|TransformX)
    (else
      (CallFunction|ReverseX))))

(event EventBeginPlay
  (bind _platform (Variables|Default|GetPlatform))
  (bind _returnvalue (Transformation|GetWorldLocation _platform))
  (Variables|Default|SetOriginX (.x _returnvalue))
  (Variables|Default|SetMoveX (+ (Variables|Default|GetMoveX) (.x _returnvalue)))
  (Utilities|Time|SetTimerbyEvent (delegate Custom|DirectionHandling) (Variables|Default|GetRefreshRate) true))

(fn ConstructionScript)